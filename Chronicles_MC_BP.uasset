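; Mod controller for the Chronicles mod that patches the game's data tables through ModDataTableOperations.
; It merges the mod's items, UI modules, recipes, feats, crafting station names and Jhebbal Sag ambush groups into their target tables.
; Map markers are cleared without replacement.
; Hints and the three loading-screen background tables are cleared, then ESC_UIModifications refills them with ESC versions, replacing rather than extending the originals.
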(event EventBeginPlay)

(event EventTick
  (params (DeltaSeconds :type Float%20%28single-precision%29)))

(fn ConstructionScript)

(fn ModDataTableOperations
  (Class|ModController|MergeDataTables "/Game/Items/ItemTable.ItemTable" "/Game/Mods/Chronicles_SM/Database/Chronicles_Items_-_DT.Chronicles_Items_-_DT")
  (Class|ModController|ClearDataTable "/Game/Systems/Map/MapMarkers.MapMarkers")
  (Class|ModController|ClearDataTable "/Game/UI/HUD/LoadingScreen/LoadingScreenBackgroundDataTable.LoadingScreenBackgroundDataTable")
  (Class|ModController|ClearDataTable "/Game/UI/HUD/LoadingScreen/OLD_LoadingScreenBackgroundDataTable.OLD_LoadingScreenBackgroundDataTable")
  (Class|ModController|ClearDataTable "/Game/UI/HUD/LoadingScreen/SIPTAH_LoadingScreenBackgroundDataTable.SIPTAH_LoadingScreenBackgroundDataTable")
  (Class|ModController|MergeDataTables "/Game/UI/UIModuleTable.UIModuleTable" "/Game/Mods/Chronicles_SM/UI_Modifications/ESC_UIModuleTable.ESC_UIModuleTable")
  (Class|ModController|ClearDataTable "/Game/UI/HUD/Hints/HintsDataTable.HintsDataTable")
  (|ESC_UIModifications)
  (Class|ModController|MergeDataTables "/Game/Items/Recipes/RecipesTable.RecipesTable" "/Game/Mods/Chronicles_SM/Database/DT_A_Recipes_Chronicles.DT_A_Recipes_Chronicles")
  (Class|ModController|MergeDataTables "/Game/Items/Feats/FeatTable.FeatTable" "/Game/Mods/Chronicles_SM/Database/DT_A_Feats_Chronicles.DT_A_Feats_Chronicles")
  (Class|ModController|MergeDataTables "/Game/Systems/Ambush/Groups/JhebbalSagAmbushGroups.JhebbalSagAmbushGroups" "/Game/Mods/Chronicles_SM/Database/JhebbalSagAmbushGroups.JhebbalSagAmbushGroups")
  (Class|ModController|MergeDataTables "/Game/Items/Crafting/CraftingStationNameTable.CraftingStationNameTable" "/Game/Mods/Chronicles_SM/Database/Chronicles_CraftingStation.Chronicles_CraftingStation"))